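; Player actor for the Runeks Cube minigame, where the player rotates a cube to match a password orientation.
; Two buttons play turn or swipe montages and tween the cube 90 degrees on X or Z, ignoring new rotations mid-tween.
; A third button or any flex input submits the cube's rotation as a quaternion to the minigame gamemode.
; After three correct submissions, input is disabled.
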(event `Submit Password`
  (bind _check (`self.check`))
  (bind _is_correct_password (`/Game/PlayerInfo/BP_MinigameRuneksCubeGamemode.Submit Player Password` (`self.Runeks Minigame`) (`self.PlayerNumber`) (`KismetMathLibrary.Conv_RotatorToQuaternion` (`SceneComponent.K2_GetComponentRotation` (`self.Cube`))) :!label _label))
  (if _is_correct_password
    (bind _output_get (set `self.check` (+ 1 _check)))
    (if (== _check 3)
      (`KismetSystemLibrary.PrintString` (`KismetStringLibrary.Conv_IntToString` _output_get))
      (`self.DisableInput` null))))

(event `EnhancedInput|/LimbitlessBluetoothPlugin/InputActions/IA_LightFlex`
  (params (ActionValue :type Boolean) (ElapsedSeconds :type "Float (double-precision)") (TriggeredSeconds :type "Float (double-precision)") (InputAction :type "InputAction Object Reference" :default "/LimbitlessBluetoothPlugin/InputActions/IA_LightFlex.IA_LightFlex"))
  (:`Triggered`
    (goto _label)))

(event `EnhancedInput|/LimbitlessBluetoothPlugin/InputActions/IA_MediumFlex`
  (params (ActionValue :type Boolean) (ElapsedSeconds :type "Float (double-precision)") (TriggeredSeconds :type "Float (double-precision)") (InputAction :type "InputAction Object Reference" :default "/LimbitlessBluetoothPlugin/InputActions/IA_MediumFlex.IA_MediumFlex"))
  (:`Triggered`
    (goto _label)))

(event `EnhancedInput|/LimbitlessBluetoothPlugin/InputActions/IA_StrongFlex`
  (params (ActionValue :type Boolean) (ElapsedSeconds :type "Float (double-precision)") (TriggeredSeconds :type "Float (double-precision)") (InputAction :type "InputAction Object Reference" :default "/LimbitlessBluetoothPlugin/InputActions/IA_StrongFlex.IA_StrongFlex"))
  (:`Triggered`
    (goto _label)))

(event `EnhancedInput|/MinigameCore/Input/IA_Button3`
  (params (ActionValue :type Boolean) (ElapsedSeconds :type "Float (double-precision)") (TriggeredSeconds :type "Float (double-precision)") (InputAction :type "InputAction Object Reference" :default "/MinigameCore/Input/IA_Button3.IA_Button3"))
  (:`Started`
    (goto _label)))

(event `self.ReceiveBeginPlay`
  (bind _asbp_minigame_runeks_cube_gamemode (cast `/Game/PlayerInfo/BP_MinigameRuneksCubeGamemode` (`self.Minigame`)))
  (set `self.Runeks Minigame` _asbp_minigame_runeks_cube_gamemode))

(event `EnhancedInput|/MinigameCore/Input/IA_Button1`
  (params (ActionValue :type Boolean) (ElapsedSeconds :type "Float (double-precision)") (TriggeredSeconds :type "Float (double-precision)") (InputAction :type "InputAction Object Reference" :default "/MinigameCore/Input/IA_Button1.IA_Button1"))
  (:`Started`
    (`self.XRotate`)))

(event `Apply Rotation`
  (params (`New Rotation` :type "Rotator Structure"))
  (set `self.Is Rotating` true)
  (bind (_asynctaskproxy _value) (`FCTweenBPActionRotator.TweenRotator` (`SceneComponent.K2_GetComponentRotation` (`self.Cube`)) `New Rotation` 0.25)
    (:`ApplyEasing`
      (`SceneComponent.K2_SetWorldRotation` (`self.Cube`) _value false false))
    (:`OnComplete`
      (set `self.Is Rotating` false))))

(event `EnhancedInput|/MinigameCore/Input/IA_Button2`
  (params (ActionValue :type Boolean) (ElapsedSeconds :type "Float (double-precision)") (TriggeredSeconds :type "Float (double-precision)") (InputAction :type "InputAction Object Reference" :default "/MinigameCore/Input/IA_Button2.IA_Button2"))
  (:`Started`
    (`self.ZRotate`)))

(fn `Set Rotation`
  (params (`New Rotation` :type "Rotator Structure"))
  (if (not (`self.Is Rotating`))
    (`self.Apply Rotation` `New Rotation`)
    (return)))

(fn `UserConstructionScript`)

(fn `XRotate`
  (`AnimInstance.Montage_Play` (`SkeletalMeshComponent.GetAnimInstance` (`self.Player`)) "/Game/Animations/ModChara_Anim_RM_Swipe_Montage.ModChara_Anim_RM_Swipe_Montage" 1.0 "MontageLength" 0.0 true)
  (`self.Set Rotation` (`KismetMathLibrary.ComposeRotators` (`SceneComponent.K2_GetComponentRotation` (`self.Cube`)) (struct :`Roll` 90.0))))

(fn `ZRotate`
  (`AnimInstance.Montage_Play` (`SkeletalMeshComponent.GetAnimInstance` (`self.Player`)) "/Game/Animations/ModChara_Anim_RM_Turn_Montage.ModChara_Anim_RM_Turn_Montage" 1.0 "MontageLength" 0.0 true)
  (`self.Set Rotation` (`KismetMathLibrary.ComposeRotators` (`SceneComponent.K2_GetComponentRotation` (`self.Cube`)) (struct :`Yaw` 90.0))))