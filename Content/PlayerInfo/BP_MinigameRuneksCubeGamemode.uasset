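; Game mode for a rune cube minigame where players race to match a shared password of cube rotations.
; On start it generates random 90-degree-step rotations and passes them to the level's BP_RunePassword actor, which shows each player's progress.
; Submissions are checked by quaternion angular distance, with correct steps scoring a point and earlier finishers earning larger completion bonuses.
; The game ends when every player completes the password.
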(event `self.ReceiveBeginPlay`
  (bind _returnvalue (`GameplayStatics.GetActorOfClass` "/Game/PlayerInfo/BP_RunePassword.BP_RunePassword_C"))
  (set `self.Password Actor` _returnvalue))

(event `self.OnMinigameStart`
  (`self.Generate Password`)
  (`/Game/PlayerInfo/BP_RunePassword.Set Password` (`self.Password Actor`) (`self.Password`))
  (for _index (range (`self.NumPlayers`))
    (`KismetArrayLibrary.Array_Set` (`self.Player Current Password Index`) _index 0 true))
  (`/Game/PlayerInfo/BP_RunePassword.Update Selections` (`self.Password Actor`) (`self.Player Current Password Index`)))

(event `self.OnMinigameReset`
  (`KismetArrayLibrary.Array_Clear` (`self.Player Current Password Index`))
  (`KismetArrayLibrary.Array_Clear` (`self.Password`))
  (set `self.Num Players Complete` 0))

(fn `Award Points`
  (params (Player :type Integer) (`Is Completed` :type Boolean))
  ; Award 1 point for each part of password completed so players who do not fully complete the password will be placed by what they've completed
  (`BasePointCounter.AddPoints` (`self.GetPointCounter`) (`local.Player`) 1)
  (if (`local.Is Completed`)
    ; Award bonus points for completing password. More bonus points are given to faster players
    (`BasePointCounter.AddPoints` (`self.GetPointCounter`) (`local.Player`) (- (`self.NumPlayers`) (`self.Num Players Complete`)))
    (`/Engine/EditorBlueprintResources/StandardMacros.IncrementInt` (`self.Num Players Complete`))))

(fn `Check All Players Complete`
  (for _array_element (`self.Player Current Password Index`)
    (if (< _array_element (`self.Password Length`))
      (return)))
  (`self.EndGame`))

(fn `Generate Password`
  (for _ (range (`self.Password Length`))
    (`KismetArrayLibrary.Array_Add` (`self.Password`) (`self.Get Random Rotation`))))

(fn `Get Random Rotation`
  (returns (Password :type "Quat Structure"))
  (return (`KismetMathLibrary.Conv_RotatorToQuaternion` (`KismetMathLibrary.MakeRotator` (`KismetMathLibrary.Conv_IntToDouble` (* (`KismetMathLibrary.RandomIntegerInRange` 0 3) 90)) (`KismetMathLibrary.Conv_IntToDouble` (* (`KismetMathLibrary.RandomIntegerInRange` 0 3) 90)) (`KismetMathLibrary.Conv_IntToDouble` (* (`KismetMathLibrary.RandomIntegerInRange` 0 3) 90))))))

(fn `Is Equal Int Vector`
  (params (A :type "IntVector Structure") (B :type "IntVector Structure"))
  (returns (Result :type Boolean))
  (return (and (== A_X B_X) (== A_Y B_Y) (== A_Z B_Z))))

(fn `Submit Player Password`
  (params (Player :type Integer) (`Player Rotation` :type "Quat Structure"))
  (returns (`Is Correct Password` :type Boolean) (`Is Complete` :type Boolean))
  (if (<= (`KismetMathLibrary.Quat_AngularDistance` (`|GetArrayItem` (`self.Password`) (`|GetArrayItem` (`self.Player Current Password Index`) (`local.Player`))) (`local.Player Rotation`)) 0.01)
    (bind _result (`/Engine/EditorBlueprintResources/StandardMacros.IncrementInt` (`|GetArrayItem` (`self.Player Current Password Index`) (`local.Player`)))
      (:`  `
        (`/Game/PlayerInfo/BP_RunePassword.Update Selections` (`self.Password Actor`) (`self.Player Current Password Index`))
        (bind _returnvalue (== _result (`self.Password Length`)))
        (`self.Award Points` (`local.Player`) _returnvalue)
        (`self.Check All Players Complete`)
        (return true _returnvalue)))
    (else
      (return false false))))

(fn `UserConstructionScript`
  (`parent.UserConstructionScript`))