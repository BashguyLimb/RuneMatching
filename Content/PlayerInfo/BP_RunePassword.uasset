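; BP_RunePassword displays a three-rune password along with markers showing which rune each of up to four players has selected.
; BeginPlay gathers the rune targets, in reverse numeric order, and the player markers into arrays.
; SetPassword encodes the password by setting each rune's world rotation.
; UpdateSelections moves each player's marker onto the selected rune, hiding markers for out-of-range selections and absent players.
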(event `self.ReceiveBeginPlay`
  (set `self.Password Runes` (`|MakeArray` (`self.PasswordTarget3`) (`self.PasswordTarget2`) (`self.PasswordTarget1`)))
  (set `self.Player Markers` (`|MakeArray` (`self.Player1Marker`) (`self.Player2Marker`) (`self.Player3Marker`) (`self.Player4Marker`)))
  (`KismetSystemLibrary.PrintString` (`KismetSystemLibrary.GetDisplayName` (`self.PasswordTarget1`))))

(fn `Set Password`
  (params (Password :type "Array of Quat Structure (by ref)"))
  (locals (`Current Rotation` :type "Quat Structure") (Index :type Integer))
  (for (_array_element _array_index) Password
    (set `local.Current Rotation` _array_element)
    (set `local.Index` _array_index)
    (if (< (`local.Index`) (`KismetArrayLibrary.Array_Length` (`self.Password Runes`)))
      (`SceneComponent.K2_SetWorldRotation` (`|GetArrayItem` (`self.Password Runes`) (`local.Index`)) (`KismetMathLibrary.Quat_Rotator` (`local.Current Rotation`)) false false))))

(fn `Update Selections`
  (params (`Player Selections` :type "Array of Integer (by ref)"))
  (locals (Player :type Integer) (Selection :type Integer))
  (for (_array_element _array_index) `Player Selections`
    (set `local.Selection` _array_element)
    (set `local.Player` _array_index)
    (`SceneComponent.SetVisibility` (`|GetArrayItem` (`self.Player Markers`) (`local.Player`)) true false)
    (if (< (`local.Selection`) (`KismetArrayLibrary.Array_Length` (`self.Password Runes`)))
      (`SceneComponent.K2_SetWorldLocation` (`|GetArrayItem` (`self.Player Markers`) (`local.Player`)) (`SceneComponent.K2_GetComponentLocation` (`|GetArrayItem` (`self.Password Runes`) (`local.Selection`))) false false)
      (else
        (`SceneComponent.SetVisibility` (`|GetArrayItem` (`self.Player Markers`) (`local.Player`)) false false))))
  (for _index (range (`KismetArrayLibrary.Array_Length` (`local.Player Selections`)) 4)
    (`SceneComponent.SetVisibility` (`|GetArrayItem` (`self.Player Markers`) _index) false false)))

(fn `UserConstructionScript`)