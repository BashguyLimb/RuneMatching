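; AI for the Runeks Cube minigame that drives a cube player to submit password rotations.
; On possession it caches the cube player and minigame gamemode.
; Each tick it prints the dot product of the cube's forward vector and the first password rotation's, submitting and Z-rotating only on an exact match.
; An unconnected older routine rotates and submits after random cooldowns, counting three correct answers before stopping.
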(event `self.ReceiveTick`
  (params (DeltaSeconds :type "Float (single-precision)"))
  (bind _as_bp_runeks_cube_player (`self.As BP Runeks Cube Player`))
  (bind _returnvalue (`KismetMathLibrary.Dot_VectorVector` (`SceneComponent.GetForwardVector` (`/Game/PlayerInfo/BP_RuneksCubePlayer.Cube` (`self.As BP Runeks Cube Player`))) (`KismetMathLibrary.GetForwardVector` (`KismetMathLibrary.Quat_Rotator` (`|GetArrayItem` (`/Game/PlayerInfo/BP_MinigameRuneksCubeGamemode.Password` (`self.As BP Minigame Runeks Cube Gamemode`)))))))
  (set `self.DistanceFromPassword` _returnvalue)
  (`KismetSystemLibrary.PrintString` (`KismetStringLibrary.Conv_DoubleToString` _returnvalue))
  (if (== (`self.DistanceFromPassword`) 1.0)
    (`/Game/PlayerInfo/BP_RuneksCubePlayer.Submit Password` _as_bp_runeks_cube_player)
    (`/Game/PlayerInfo/BP_RuneksCubePlayer.ZRotate` _as_bp_runeks_cube_player)))

(event `self.OnMinigamePlayerPossessed`
  (bind _asbp_runeks_cube_player (cast `/Game/PlayerInfo/BP_RuneksCubePlayer` (`self.Player`)))
  (set `self.As BP Runeks Cube Player` _asbp_runeks_cube_player)
  (bind _asbp_minigame_runeks_cube_gamemode (cast `/Game/PlayerInfo/BP_MinigameRuneksCubeGamemode` (`GameplayStatics.GetGameMode`)))
  (set `self.As BP Minigame Runeks Cube Gamemode` _asbp_minigame_runeks_cube_gamemode))

(fn `UserConstructionScript`)